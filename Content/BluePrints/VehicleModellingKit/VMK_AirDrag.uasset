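; Vehicle Modelling Kit component that applies aerodynamic drag to the owning vehicle's chassis, found by static mesh component name at BeginPlay.
; Each Tick, unless SleepMod is set, it computes a force opposing the owner's velocity from the quadratic drag equation, using km/h speed rescaled to Unreal units.
; ApplyAtOwnLocation selects whether the force acts at the component's location or on the chassis body, with optional debug drawing.
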(event EventBeginPlay
  (CallFunction|GetChassisReference))

(event EventTick
  (params (DeltaSeconds :type Float%20%28single-precision%29))
  (if (Variables|Default|GetSleepMod)
    (if (Variables|Default|GetDebugMod)
      (Rendering|Debug|DrawDebugString (Transformation|GetWorldLocation) "Sleeping..." 0 "(R=1.000000,G=1.000000,B=1.000000,A=1.000000)"))
    (else
      (CallFunction|AddAirDrag))))

(fn AddAirDrag
  (bind _returnvalue (Transformation|GetWorldLocation))
  (bind _returnvalue_2 (Components|GetOwner))
  (bind _chassis (Variables|Components|GetChassis))
  (bind _airdensity (Variables|Default|GetAirDensity))
  (bind _dragcoef (Variables|Default|GetDragCoef))
  (bind _dragsurfacearea (Variables|Default|GetDragSurfaceArea))
  (bind _returnvalue_3 (Transformation|GetVelocity _returnvalue_2))
  (bind _returnvalue_4 (Math|Vector|VectorLength _returnvalue_3))
  (bind _returnvalue_5 (Math|Vector|Normalize _returnvalue_3))
  (bind _returnvalue_6 (* _returnvalue_5 -1.0))
  (bind _returnvalue_7 (* _returnvalue_4 0.036))
  (bind _returnvalue_8 (* _returnvalue_7 _returnvalue_7 _airdensity _dragsurfacearea _dragcoef 0.5))
  (bind _returnvalue_9 (* _returnvalue_8 27.7777778))
  (bind _returnvalue_10 (* _returnvalue_6 _returnvalue_9))
  (if (Variables|Default|GetApplyAtOwnLocation)
    (Class|PrimitiveComponent|AddForceatLocation _chassis _returnvalue_10 (Transformation|GetWorldLocation) "None")
    (if (Variables|Default|GetDebugMod)
      (Rendering|Debug|DrawDebugLine _returnvalue (+ _returnvalue (* _returnvalue_10 0.01)) "(R=0.945000,G=0.539004,B=0.259891,A=1.000000)" 0.0 5.0))
    (else
      (Physics|AddForce _chassis _returnvalue_10 "None" false)
      (if (Variables|Default|GetDebugMod)
        (bind _returnvalue_11 (Physics|GetCenterOfMass (Variables|Components|GetChassis) "None"))
        (Rendering|Debug|DrawDebugLine _returnvalue_11 (+ _returnvalue_11 (* _returnvalue_10 0.01)) "(R=0.945000,G=0.539004,B=0.259891,A=1.000000)" 0.0 5.0)))))

(fn GetChassisReference
  (for _array_element (Actor|GetComponentsByClass (Components|GetOwner) "/Script/Engine.StaticMeshComponent")
    (if (Utilities|Enum|Equal(Enum) (Utilities|GetObjectName _array_element) (Variables|Default|GetChasisComponentName))
      (Variables|Components|SetChassis _array_element)))
  (Utilities|IsValid (Variables|Components|GetChassis)
    (:Is%20Not%20Valid
      (Development|PrintString "Chassis reference is not valid in Suspension component!" true true "(R=1.000000,G=0.000000,B=0.064224,A=1.000000)" 1e+01))))