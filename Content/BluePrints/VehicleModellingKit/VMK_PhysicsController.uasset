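; VMK_PhysicsController is a Vehicle Modelling Kit component that keeps a registry of its owning actor's scene components.
; On BeginPlay it gathers every other SceneComponent on the owner into the NamedComponents array.
; Helper functions find a component's index by object name, return the reference at an index, and print the registered names for debugging.
; Despite its name, it contains no physics logic and Tick is unused.
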(event EventBeginPlay
  (|CallParentFunction)
  (CallFunction|RegisterComponents))

(event EventTick
  (params (DeltaSeconds :type Float%20%28single-precision%29)))

(fn RegisterComponents
  (for _array_element (Actor|GetComponentsByClass (Components|GetOwner) "/Script/Engine.SceneComponent")
    (if (!= _array_element self)
      (Utilities|Array|AddUnique (Variables|Default|GetNamed_Components) _array_element))))

(fn LogRegisteredComponents
  (Development|PrintString "Components registered: " true true "(R=1.000000,G=0.910999,B=0.155962,A=1.000000)" 5.0)
  (for _array_element (Variables|Default|GetNamed_Components)
    (Development|PrintString (Utilities|GetObjectName _array_element) true true "(R=1.000000,G=0.910999,B=0.155962,A=1.000000)" 5.0)))

(fn GetComponentIndexbyName
  (params (ComponentName :type String))
  (for (_array_element _array_index) (Variables|Default|GetNamed_Components)
    (if (Utilities|Enum|Equal(Enum) (Utilities|GetObjectName _array_element) ComponentName)
      (LocalVariables|SetLSuccess true)
      (LocalVariables|SetLIndex _array_index)))
  (return (LocalVariables|GetLSuccess) (LocalVariables|GetLIndex)))

(fn GetComponentReferencebyIndex
  (params (ComponentIndex :type Integer))
  (if (>= ComponentIndex 0)
    (LocalVariables|SetComponent (Utilities|Array|Get(acopy) (Variables|Default|GetNamed_Components) ComponentIndex)))
  (return (LocalVariables|GetComponent)))