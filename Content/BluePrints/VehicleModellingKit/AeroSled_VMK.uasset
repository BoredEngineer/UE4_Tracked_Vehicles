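; Physics-driven, player-controlled aerosled from the Vehicle Modelling Kit, with a propeller engine and four suspended skis.
; Forward input drives the thruster, reverse engages rear brakes, and steering interpolates the front skis' constraint yaw targets.
; Ski hits count valid contacts, which feed each suspension's friction on Tick.
; After a delay at low velocity, bodies and kit components sleep until input or motion wakes them; debug toggling and camera zoom are included.
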(event OnComponentHit(Ski_RF)
  (params (OtherActor :type Actor%20Object%20Reference) (OtherComp :type Primitive%20Component%20Object%20Reference) (NormalImpulse :type Vector :default "0, 0, 0") (Hit :type Hit%20Result%20Structure%20%28by%20ref%29))
  (bind _validpoint_ (Default|TestPointValidity (Variables|Default|GetSusp_RF)))
  (if _validpoint_
    (Math|Float|IncrementFloat (Variables|Default|GetNumValidColliders))))

(event OnComponentHit(Ski_LF)
  (params (OtherActor :type Actor%20Object%20Reference) (OtherComp :type Primitive%20Component%20Object%20Reference) (NormalImpulse :type Vector :default "0, 0, 0") (Hit :type Hit%20Result%20Structure%20%28by%20ref%29))
  (bind _validpoint_ (Default|TestPointValidity (Variables|Default|GetSusp_LF)))
  (if _validpoint_
    (Math|Float|IncrementFloat (Variables|Default|GetNumValidColliders))))

(event OnComponentHit(Ski_RB)
  (params (OtherActor :type Actor%20Object%20Reference) (OtherComp :type Primitive%20Component%20Object%20Reference) (NormalImpulse :type Vector :default "0, 0, 0") (Hit :type Hit%20Result%20Structure%20%28by%20ref%29))
  (bind _validpoint_ (Default|TestPointValidity (Variables|Default|GetSusp_RB)))
  (if _validpoint_
    (Math|Float|IncrementFloat (Variables|Default|GetNumValidColliders))))

(event OnComponentHit(Ski_LB)
  (params (OtherActor :type Actor%20Object%20Reference) (OtherComp :type Primitive%20Component%20Object%20Reference) (NormalImpulse :type Vector :default "0, 0, 0") (Hit :type Hit%20Result%20Structure%20%28by%20ref%29))
  (bind _validpoint_ (Default|TestPointValidity (Variables|Default|GetSusp_LB)))
  (if _validpoint_
    (Math|Float|IncrementFloat (Variables|Default|GetNumValidColliders))))

(event EventBeginPlay)

(event Collision|EventActorBeginOverlap
  (params (OtherActor :type Actor%20Object%20Reference)))

(event EventTick
  (params (DeltaSeconds :type Float%20%28single-precision%29))
  (bind _sleeping_ (CallFunction|PuttoSleep))
  (if (not _sleeping_)
    (Utilities|FlowControl|Sequence
      (:then_0
        (Default|ApplyFriction :self (Variables|Default|GetSusp_LF) :NumOfContactPoints (Variables|Default|GetNumValidColliders))
        (Variables|Default|SetNumValidColliders 0.0)
        (CallFunction|ProcessSteering))
      (:then_1
        (if (Variables|Default|GetDebug)
          (bind _returnvalue (Physics|GetCenterOfMass (Variables|Default|GetChassis) "None"))
          (Rendering|Debug|DrawDebugString _returnvalue (Utilities|String|ToString(Vector) (Math|Transform|InverseTransformLocation (Transformation|GetActorTransform) _returnvalue)) 0 "(R=0.029521,G=0.000000,B=1.000000,A=1.000000)"))))))

(event Input|ActionEvents|InputActionDebugMode
  (params (Key :type Key%20Structure :default "AnyKey"))
  ;[1 1 1] Switch Debug mode
  (:Pressed
    (Utilities|FlowControl|FlipFlop
      (:A
        (Variables|Default|SetDebug true)
        (CallFunction|SwitchDebugonComponents true))
      (:B
        (Variables|Default|SetDebug false)
        (CallFunction|SwitchDebugonComponents false)))))

(event Input|ActionEvents|InputActionZoomIn
  (params (Key :type Key%20Structure :default "AnyKey"))
  (bind _springarm (Variables|Default|GetSpringArm))
  ;[1 1 1] Camera Control
  (:Pressed
    (Variables|/Script/Engine.SpringArmComponent|SetTargetArmLength _springarm (+ (Variables|/Script/Engine.SpringArmComponent|GetTargetArmLength _springarm) -25.0))))

(event Input|ActionEvents|InputActionZoomOut
  (params (Key :type Key%20Structure :default "AnyKey"))
  (bind _springarm (Variables|Default|GetSpringArm))
  ;[1 1 1] Camera Control
  (:Pressed
    (Variables|/Script/Engine.SpringArmComponent|SetTargetArmLength _springarm (+ (Variables|/Script/Engine.SpringArmComponent|GetTargetArmLength _springarm) 25.0))))

(event Input|AxisEvents|InputAxisVehicleForwardBackward
  (params (AxisValue :type Float%20%28single-precision%29))
  (Default|SetThrusteronOff (Variables|Default|GetVMK_PropellerEngine) AxisValue)
  (Default|EngageBreaks (Variables|Default|GetSusp_LB) (select (< AxisValue 0.0) true false))
  (if (and (or (!= AxisValue 0.0) (!= (stale Input|AxisEvents|InputAxisVehicleRightLeft AxisValue) 0.0)) (Variables|Default|GetSleepMod))
    (Variables|Default|SetSleepMod false)
    (CallFunction|PutComponentstoSleep false)
    (Variables|Default|SetSleepDelayTimer 0.0)))

(event Input|AxisEvents|InputAxisVehicleRightLeft
  (params (AxisValue :type Float%20%28single-precision%29))
  (Variables|Default|SetSteerRatio (* AxisValue -1.0))
  (if (and (or (!= (stale Input|AxisEvents|InputAxisVehicleForwardBackward AxisValue) 0.0) (!= AxisValue 0.0)) (Variables|Default|GetSleepMod))
    (Variables|Default|SetSleepMod false)
    (CallFunction|PutComponentstoSleep false)
    (Variables|Default|SetSleepDelayTimer 0.0)))

(event Input|KeyboardEvents|G
  (params (Key :type Key%20Structure :default "AnyKey"))
  (:Pressed
    (bind _scenecomponent (Default|GetComponentReferencebyIndex (Variables|Default|GetVMK_PhysicsController) (Variables|/Game/BluePrints/VehicleModellingKit/VMK_PropellerEngine.VMK_PropellerEngine_C|GetChassis_VMK_index (Variables|Default|GetVMK_PropellerEngine))))
    (Development|PrintString (Utilities|GetObjectName _scenecomponent))))

(event Input|KeyboardEvents|H
  (params (Key :type Key%20Structure :default "AnyKey"))
  (:Pressed
    (Default|LogRegisteredComponents (Variables|Default|GetVMK_PhysicsController))))

(fn ConstructionScript
  (bind _returnvalue (Physics|GetCenterOfMass (Variables|Default|GetChassis) "None"))
  (Transformation|SetRelativeLocation (Variables|Default|GetCOM) (Math|Transform|InverseTransformLocation (Transformation|GetActorTransform) _returnvalue) false false))

(fn ProcessSteering
  (Variables|Default|SetCurrentSteeringYaw (Math|Interpolation|FInterptoConstant (Variables|Default|GetCurrentSteeringYaw) (* (Variables|Default|GetSteerRatio) (Variables|Default|GetMaxSteeringAngle)) (Utilities|Time|GetWorldDeltaSeconds) 2e+01))
  (Utilities|FlowControl|Sequence
    (:then_0
      (Class|PhysicsConstraintComponent|SetAngularOrientationTarget (Variables|Default|GetSki_RF_PC) (Math|Rotator|MakeRotator 0.0 0.0 (Variables|Default|GetCurrentSteeringYaw))))))

(fn AllignSpring
  (params (Spring :type Static%20Mesh%20Component%20Object%20Reference) (Suspension :type Suspension%20Object%20Reference) (Ski :type Static%20Mesh%20Component%20Object%20Reference))
  (bind _returnvalue (Transformation|GetWorldLocation Suspension))
  (bind _returnvalue_2 (Transformation|GetWorldLocation Ski))
  (bind _relativescale3d (Variables|/Script/Engine.SceneComponent|GetRelativeScale3D Spring))
  (Transformation|SetWorldLocationAndRotation Spring _returnvalue (Math|Rotator|FindLookatRotation _returnvalue _returnvalue_2) false false)
  (Transformation|SetRelativeScale3D Spring (Math|Vector|MakeVector (/ (Math|Vector|VectorLength (- _returnvalue _returnvalue_2)) 1e+02) (.y _relativescale3d) (.z _relativescale3d))))

(fn PuttoSleep
  (bind _chassis (Variables|Default|GetChassis))
  (bind _sleepvelocity (Variables|Default|GetSleepVelocity))
  (if (Variables|Default|GetSleepMod)
    (bind _returnvalue (Physics|GetPhysicsLinearVelocity _chassis "None" :!label _label))
    (bind _returnvalue_2 (Class|PrimitiveComponent|GetPhysicsAngularVelocity _chassis "None"))
    (if (and (< (Math|Vector|VectorLength _returnvalue) _sleepvelocity) (< (Math|Vector|VectorLength _returnvalue_2) _sleepvelocity))
      (if (not (Variables|Default|GetSleepMod))
        (Variables|Default|SetSleepMod true)
        (CallFunction|PutComponentstoSleep true))
      (elif (Variables|Default|GetSleepMod)
        (Variables|Default|SetSleepMod false)
        (CallFunction|PutComponentstoSleep false)
        (Variables|Default|SetSleepDelayTimer 0.0)))
    (else
      (Math|Float|CompareFloat (Variables|Default|GetSleepDelayTimer) (Variables|Default|GetSleepTimerSeconds)
        (:>
          (goto _label))
        (:==
          (goto _label))
        (:<
          (Variables|Default|SetSleepDelayTimer (+ (Variables|Default|GetSleepDelayTimer) (Utilities|Time|GetWorldDeltaSeconds)))))))
  (return (Variables|Default|GetSleepMod)))

(fn PutComponentstoSleep
  (params (SleepMod :type Boolean))
  (Class|PrimitiveComponent|PutRigidBodytoSleep (Actor|GetComponentsByClass "/Script/Engine.StaticMeshComponent") "None")
  (for _array_element (Components|GetChildrenComponents (Variables|Default|GetChassis) true)
    (if (Utilities|DoesObjectImplementInterface _array_element "/Game/BluePrints/Interfaces/SleepMod.SleepMod_C")
      (Class|SleepMod|SwitchSleepMod(Message) _array_element SleepMod)
      (elif (Utilities|DoesObjectImplementInterface _array_element "/Game/BluePrints/VehicleModellingKit/VMK_BaseInterface.VMK_BaseInterface_C")
        (Class|VMKBaseInterface|SwitchSleepMod(Message) _array_element SleepMod)))))

(fn SwitchDebugonComponents
  (params (DebugMod :type Boolean))
  (for _array_element (Actor|GetComponentsByClass "/Game/BluePrints/VehicleModellingKit/VMK_BaseComponent.VMK_BaseComponent_C")
    (Default|SwitchDebugMod _array_element DebugMod)))