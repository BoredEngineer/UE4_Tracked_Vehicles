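; Base component of the Vehicle Modelling Kit that gives vehicle parts a link to their owner's VMK_PhysicsController.
; On BeginPlay it searches the owner for that controller, caches it and prints an on-screen warning if none exists.
; Name-to-index lookups are forwarded to the controller, with error prints on failure.
; Setters store debug and sleep flags, while the transform-by-index getter is an empty stub.
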(event EventBeginPlay
  (CallFunction|GetReferencetoVMKPhysicsController))

(event EventTick
  (params (DeltaSeconds :type Float%20%28single-precision%29)))

(fn GetReferencetoVMKPhysicsController
  (for _array_element (Actor|GetComponentsByClass (Components|GetOwner) "/Game/BluePrints/VehicleModellingKit/VMK_PhysicsController.VMK_PhysicsController_C")
    (Utilities|IsValid _array_element
      (:Is%20Valid
        (Variables|Default|SetVMK_PhysicsController _array_element))))
  (Utilities|IsValid (Variables|Default|GetVMK_PhysicsController)
    (:Is%20Not%20Valid
      (Development|PrintString "VMK Physics Controller not detected!" true true "(R=1.000000,G=0.000000,B=0.028928,A=1.000000)" 5.0))))

(fn GetComponentIndexbyName
  (params (Name :type String))
  (bind _vmk_physicscontroller (Variables|Default|GetVMK_PhysicsController))
  (Utilities|IsValid _vmk_physicscontroller
    (:Is%20Valid
      (bind (_found_ _index) (Default|GetComponentIndexbyName _vmk_physicscontroller Name))
      (if _found_
        (LocalVariables|SetIndex _index)
        (else
          (Development|PrintString (Utilities|String|Append (Utilities|GetObjectName self) "->GetComponentIndexByName" " \"No component found by this name!\"") true true "(R=1.000000,G=0.000000,B=0.062745,A=1.000000)" 5.0))))
    (:Is%20Not%20Valid
      (Development|PrintString (Utilities|String|Append (Utilities|GetObjectName self) "->GetComponentIndexByName" " \"No valid VMK Physics Controller found!\"") true true "(R=1.000000,G=0.000000,B=0.062745,A=1.000000)" 5.0)))
  (return (LocalVariables|GetIndex)))

(fn GetComponentTransformbyIndex
  (params (CompIndex :type Integer))
  (return ""))

(fn SwitchDebugMod
  (params (Debug :type Boolean))
  (Variables|Default|SetDebugMod Debug)
  (return false))

(fn SwitchSleepMod
  (params (Sleep :type Boolean))
  (Variables|Default|SetSleepMod Sleep)
  (return false))