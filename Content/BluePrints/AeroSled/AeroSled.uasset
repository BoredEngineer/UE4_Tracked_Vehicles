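; AeroSled is a player-controlled, thruster-driven sled on four physics skis with suspension components.
; Valid ski hits are counted and fed each tick into every suspension's friction, then the count resets.
; Forward/back input drives the thruster and rear brakes, while left/right yaws front constraint targets to steer.
; Zoom inputs change spring arm length, and construction moves a COM marker to the chassis center of mass.
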(event OnComponentHit(Ski_RF)
  (params (OtherActor :type Actor%20Object%20Reference) (OtherComp :type Primitive%20Component%20Object%20Reference) (NormalImpulse :type Vector :default "0, 0, 0") (Hit :type Hit%20Result%20Structure%20%28by%20ref%29))
  (bind _validpoint_ (Default|TestPointValidity (Variables|Default|GetSusp_RF)))
  (if _validpoint_
    (Math|Float|IncrementFloat (Variables|Default|GetNumValidColliders))))

(event OnComponentHit(Ski_LF)
  (params (OtherActor :type Actor%20Object%20Reference) (OtherComp :type Primitive%20Component%20Object%20Reference) (NormalImpulse :type Vector :default "0, 0, 0") (Hit :type Hit%20Result%20Structure%20%28by%20ref%29))
  (bind _validpoint_ (Default|TestPointValidity (Variables|Default|GetSusp_LF)))
  (if _validpoint_
    (Math|Float|IncrementFloat (Variables|Default|GetNumValidColliders))))

(event OnComponentHit(Ski_RB)
  (params (OtherActor :type Actor%20Object%20Reference) (OtherComp :type Primitive%20Component%20Object%20Reference) (NormalImpulse :type Vector :default "0, 0, 0") (Hit :type Hit%20Result%20Structure%20%28by%20ref%29))
  (bind _validpoint_ (Default|TestPointValidity (Variables|Default|GetSusp_RB)))
  (if _validpoint_
    (Math|Float|IncrementFloat (Variables|Default|GetNumValidColliders))))

(event OnComponentHit(Ski_LB)
  (params (OtherActor :type Actor%20Object%20Reference) (OtherComp :type Primitive%20Component%20Object%20Reference) (NormalImpulse :type Vector :default "0, 0, 0") (Hit :type Hit%20Result%20Structure%20%28by%20ref%29))
  (bind _validpoint_ (Default|TestPointValidity (Variables|Default|GetSusp_LB)))
  (if _validpoint_
    (Math|Float|IncrementFloat (Variables|Default|GetNumValidColliders))))

(event EventBeginPlay)

(event EventActorBeginOverlap
  (params (OtherActor :type Actor%20Object%20Reference)))

(event EventTick
  (params (DeltaSeconds :type Float%20%28single-precision%29))
  (Utilities|FlowControl|Sequence
    (:then_0
      (Default|ApplyFriction :self (Variables|Default|GetSusp_LF) :NumOfContactPoints (Variables|Default|GetNumValidColliders))
      (Variables|Default|SetNumValidColliders 0.0))
    (:then_1
      (if (Variables|Default|GetDebug)
        (bind _returnvalue (Physics|GetCenterOfMass (Variables|Default|GetChassis) "None"))
        (Rendering|Debug|DrawDebugString _returnvalue (Utilities|String|ToString(Vector) (Math|Transform|InverseTransformLocation (Transformation|GetActorTransform) _returnvalue)) 0 "(R=0.029521,G=0.000000,B=1.000000,A=1.000000)")))))

(event Input|ActionEvents|InputActionZoomIn
  (params (Key :type Key%20Structure :default "AnyKey"))
  (bind _springarm (Variables|Default|GetSpringArm))
  ;[1 1 1] Camera Control
  (:Pressed
    (Variables|/Script/Engine.SpringArmComponent|SetTargetArmLength _springarm (+ (Variables|/Script/Engine.SpringArmComponent|GetTargetArmLength _springarm) -25.0))))

(event Input|ActionEvents|InputActionZoomOut
  (params (Key :type Key%20Structure :default "AnyKey"))
  (bind _springarm (Variables|Default|GetSpringArm))
  ;[1 1 1] Camera Control
  (:Pressed
    (Variables|/Script/Engine.SpringArmComponent|SetTargetArmLength _springarm (+ (Variables|/Script/Engine.SpringArmComponent|GetTargetArmLength _springarm) 25.0))))

(event Input|AxisEvents|InputAxisVehicleForwardBackward
  (params (AxisValue :type Float%20%28single-precision%29))
  (Default|SetThrusteronOff (Variables|Default|GetThruster) AxisValue)
  (Default|EngageBreaks (Variables|Default|GetSusp_LB) (select (< AxisValue 0.0) true false)))

(event Input|AxisEvents|InputAxisVehicleRightLeft
  (params (AxisValue :type Float%20%28single-precision%29))
  (Utilities|FlowControl|Sequence
    (:then_0
      (Class|PhysicsConstraintComponent|SetAngularOrientationTarget (Variables|Default|GetP_LF) (Math|Rotator|MakeRotator 0.0 0.0 (* (* AxisValue 15.0) -1.0))))))

(fn ConstructionScript
  (bind _returnvalue (Physics|GetCenterOfMass (Variables|Default|GetChassis) "None"))
  (Transformation|SetRelativeLocation (Variables|Default|GetCOM) (Math|Transform|InverseTransformLocation (Transformation|GetActorTransform) _returnvalue) false false))