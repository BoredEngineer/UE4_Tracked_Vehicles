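; Thruster component for the AeroSled that pushes the owner's chassis mesh along the component's forward vector.
; At BeginPlay it finds the chassis static mesh by name, then each Tick applies force at its own location, producing off-center torque when offset.
; SetThrusterOnOff stores a ratio used only as an on/off switch: throttle ramps up gradually while positive and falls faster otherwise, scaling thruster power.
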(event EventBeginPlay
  (CallFunction|GetChassisReference))

(event EventTick
  (params (DeltaSeconds :type Float%20%28single-precision%29))
  (CallFunction|UpdateThrust)
  (CallFunction|ApplyThrust))

(fn GetChassisReference
  (for _array_element (Actor|GetComponentsByClass (Components|GetOwner) "/Script/Engine.StaticMeshComponent")
    (if (Utilities|Enum|Equal(Enum) (Utilities|GetObjectName _array_element) (Variables|Default|GetChasisComponentName))
      (Variables|Default|SetChassis _array_element)))
  (Utilities|IsValid (Variables|Default|GetChassis)
    (:Is%20Not%20Valid
      (Development|PrintString "Chassis reference is not valid in Suspension component!" true true "(R=1.000000,G=0.000000,B=0.064224,A=1.000000)" 1e+01))))

(fn ApplyThrust
  (Class|PrimitiveComponent|AddForceatLocation (Variables|Default|GetChassis) (Variables|Default|GetThrustForce) (Transformation|GetWorldLocation) "None"))

(fn UpdateThrust
  (bind _returnvalue (Transformation|GetWorldLocation))
  (Variables|Default|SetThrottle (Math|Float|Clamp(Float) (+ (Variables|Default|GetThrottle) (* (Math|Float|SelectFloat 0.5 -1.0 (> (Variables|Default|GetThrusterRatio) 0.0)) (Utilities|Time|GetWorldDeltaSeconds)))))
  (Variables|Default|SetThrustForce (* (Math|Vector|GetForwardVector) (* (Variables|Default|GetThrottle) (Variables|Default|GetThrusterPower))))
  (if (Variables|Default|GetDebug)
    (Rendering|Debug|DrawDebugLine :LineStart _returnvalue :LineEnd (+ _returnvalue (* (Math|Vector|GetForwardVector) (* (Variables|Default|GetThrottle) (Variables|Default|GetThrusterPower)))) :Thickness 5.0)
    (Rendering|Debug|DrawDebugString (Transformation|GetWorldLocation) (Utilities|String|Append "Throttle: " (Utilities|String|ToString(Float) (Variables|Default|GetThrottle))) 0 "(R=1.000000,G=1.000000,B=1.000000,A=1.000000)")))

(fn SetThrusteronOff
  (params (ThrusterRatio :type Float%20%28single-precision%29))
  (Variables|Default|SetThrusterRatio ThrusterRatio)
  (return false))