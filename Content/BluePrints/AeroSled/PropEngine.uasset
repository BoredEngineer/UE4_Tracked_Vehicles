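; Propeller engine scene component for the AeroSled that pushes the chassis along the component's forward vector and spins the propeller mesh.
; It finds both meshes on its owner by name at BeginPlay.
; Each tick, a positive ThrusterRatio ramps Throttle up, otherwise down faster, and a curve converts it into force applied at the component's location.
; Sleep mode skips thrust updates while the throttle-based propeller spin continues, with optional debug drawing.
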(event EventBeginPlay
  (CallFunction|GetChassisReference))

(event EventTick
  (params (DeltaSeconds :type Float%20%28single-precision%29))
  (CallFunction|AnimatePropeller)
  (if (Variables|Default|GetSleepMod)
    (if (Variables|Default|GetDebug?)
      (Rendering|Debug|DrawDebugString (Transformation|GetWorldLocation) "Sleeping..." 0 "(R=1.000000,G=1.000000,B=1.000000,A=1.000000)"))
    (else
      (CallFunction|UpdateThrust)
      (CallFunction|ApplyThrust))))

(fn GetChassisReference
  (for _array_element (Actor|GetComponentsByClass (Components|GetOwner) "/Script/Engine.StaticMeshComponent")
    (if (Utilities|Enum|Equal(Enum) (Utilities|GetObjectName _array_element) (Variables|Default|GetChasisComponentName))
      (Variables|Default|SetChassis _array_element)
      (elif (Utilities|Enum|Equal(Enum) (Utilities|GetObjectName _array_element) (Variables|Default|GetPropellerMeshName))
        (Variables|Default|SetPropeller _array_element))))
  (Utilities|FlowControl|Sequence
    (:then_0
      (Utilities|IsValid (Variables|Default|GetChassis)
        (:Is%20Not%20Valid
          (Development|PrintString "Chassis reference is not valid in Suspension component!" true true "(R=1.000000,G=0.000000,B=0.064224,A=1.000000)" 1e+01))))
    (:then_1
      (Utilities|IsValid (Variables|Default|GetPropeller)
        (:Is%20Not%20Valid
          (Development|PrintString "Propeller reference is not valid in Suspension component!" true true "(R=1.000000,G=0.000000,B=0.064224,A=1.000000)" 1e+01))))))

(fn ApplyThrust
  (Class|PrimitiveComponent|AddForceatLocation (Variables|Default|GetChassis) (Variables|Default|GetThrustForce) (Transformation|GetWorldLocation) "None"))

(fn UpdateThrust
  (bind _returnvalue (Transformation|GetWorldLocation))
  (Variables|Default|SetThrottle (Math|Float|Clamp(Float) (+ (Variables|Default|GetThrottle) (* (Math|Float|SelectFloat 0.5 -1.0 (> (Variables|Default|GetThrusterRatio) 0.0)) (Utilities|Time|GetWorldDeltaSeconds)))))
  (Variables|Default|SetThrustForce (* (Math|Vector|GetForwardVector) (* (Math|Curves|GetFloatValue (Variables|Default|GetThrottleCurve) (Variables|Default|GetThrottle)) (Variables|Default|GetThrusterPower))))
  (if (Variables|Default|GetDebug?)
    (Rendering|Debug|DrawDebugLine :LineStart _returnvalue :LineEnd (+ _returnvalue (* (Math|Vector|GetForwardVector) (* (Math|Curves|GetFloatValue (Variables|Default|GetThrottleCurve) (Variables|Default|GetThrottle)) (Variables|Default|GetThrusterPower)))) :Thickness 5.0)
    (Rendering|Debug|DrawDebugString (Transformation|GetWorldLocation) (Utilities|String|Append "Throttle: " (Utilities|String|ToString(Float) (Variables|Default|GetThrottle))) 0 "(R=1.000000,G=1.000000,B=1.000000,A=1.000000)")))

(fn SetThrusteronOff
  (params (ThrusterRatio :type Float%20%28single-precision%29))
  (Variables|Default|SetThrusterRatio ThrusterRatio)
  (return false))

(fn AnimatePropeller
  (Transformation|AddLocalRotation (Variables|Default|GetPropeller) (Math|Rotator|MakeRotator (* (Math|Float|Lerp (Variables|Default|GetMinPropVelocity) (Variables|Default|GetMaxPropVelocity) (Variables|Default|GetThrottle)) -1.0) 0.0 0.0) false false))

(fn SwitchSleepMod
  (params (SleepMod :type Boolean))
  (Variables|Default|SetSleepMod SleepMod)
  (return false))