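; Actor component that applies aerodynamic drag to its owner, likely an AeroSled vehicle.
; On BeginPlay it finds the owner's chassis static mesh component by name.
; Each tick it computes quadratic drag from speed converted to km/h, air density, surface area and drag coefficient, then scales it to Unreal units.
; It applies that force against the velocity and draws it as a debug line from the center of mass.
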(event EventBeginPlay
  (CallFunction|GetChassisReference))

(event EventTick
  (params (DeltaSeconds :type Float%20%28single-precision%29))
  (CallFunction|AddAirDrag))

(fn AddAirDrag
  (bind _returnvalue (Components|GetOwner))
  (bind _airdensity (Variables|Default|GetAirDensity))
  (bind _dragcoef (Variables|Default|GetDragCoef))
  (bind _dragsurfacearea (Variables|Default|GetDragSurfaceArea))
  (bind _returnvalue_2 (Transformation|GetVelocity _returnvalue))
  (bind _returnvalue_3 (Math|Vector|VectorLength _returnvalue_2))
  (bind _returnvalue_4 (Math|Vector|Normalize _returnvalue_2))
  (bind _returnvalue_5 (* _returnvalue_4 -1.0))
  (bind _returnvalue_6 (* _returnvalue_3 0.036))
  (bind _returnvalue_7 (* _returnvalue_6 _returnvalue_6 _airdensity _dragsurfacearea _dragcoef 0.5))
  (bind _returnvalue_8 (* _returnvalue_7 27.7777778))
  (bind _returnvalue_9 (* _returnvalue_5 _returnvalue_8))
  (Physics|AddForce (Variables|Components|GetChassis) _returnvalue_9 "None" false)
  (bind _returnvalue_10 (Physics|GetCenterOfMass (Variables|Components|GetChassis) "None"))
  (Rendering|Debug|DrawDebugLine _returnvalue_10 (+ _returnvalue_10 (* _returnvalue_9 0.001)) "(R=0.945000,G=0.539004,B=0.259891,A=1.000000)" 0.0 5.0))

(fn GetChassisReference
  (for _array_element (Actor|GetComponentsByClass (Components|GetOwner) "/Script/Engine.StaticMeshComponent")
    (if (Utilities|Enum|Equal(Enum) (Utilities|GetObjectName _array_element) (Variables|Default|GetChasisComponentName))
      (Variables|Components|SetChassis _array_element)
      (Development|PrintString "Found Chassis"))))