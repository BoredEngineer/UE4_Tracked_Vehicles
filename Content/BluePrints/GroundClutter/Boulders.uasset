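; Boulders is a ground clutter Blueprint that scatters physics-driven copies of a static mesh, presumably boulders, around the actor.
; The construction script adds mesh components at random X/Y offsets within Spacing and random rotations, using Amount, Scale and StaticMesh, and stores them in Collection.
; On BeginPlay, every stored component starts simulating physics with a raised mass scale.
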(event EventBeginPlay
  (for _array_element (Variables|Default|GetCollection)
    (Physics|SetSimulatePhysics _array_element true)
    (Class|PrimitiveComponent|SetMassScale _array_element "None" 2e+01)))

(event Collision|EventActorBeginOverlap
  (params (OtherActor :type Actor%20Object%20Reference)))

(event EventTick
  (params (DeltaSeconds :type Float%20%28single-precision%29)))

(fn ConstructionScript
  (bind _spacing (Variables|Default|GetSpacing))
  (bind _returnvalue (* _spacing -1.0))
  (for _index (range 0 (Variables|Default|GetAmount))
    (bind _returnvalue_2 (AddComponent|AddStaticMeshComponent false (Math|Transform|MakeTransform (Math|Vector|MakeVector (Math|Random|RandomFloatinRange _returnvalue _spacing) (Math|Random|RandomFloatinRange _returnvalue _spacing) 0.0) (Math|Random|RandomRotator false) (Variables|Default|GetScale))))
    (Components|StaticMesh|SetStaticMesh _returnvalue_2 (Variables|Default|GetStaticMesh))
    (Utilities|Array|Add (Variables|Default|GetCollection) _returnvalue_2)))