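; Test physics box for experimenting with friction by switching physical materials on contact, with camera zoom and velocity debug text.
; H pushes the Cube at point F, and B brakes it with velocity-cancelling forces spread over T1–T4.
; Hits on P1–P4 draw contact points and call ApplyFriction, which leaves that part on NoFric_V2 and the Cube on FullFric.
; A manual clamped friction-force calculation and other force experiments remain disconnected.
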(event OnComponentHit(P2)
  (params (OtherActor :type Actor%20Object%20Reference) (OtherComp :type Primitive%20Component%20Object%20Reference) (NormalImpulse :type Vector) (Hit :type Hit%20Result%20Structure%20%28by%20ref%29))
  (if (.bblockinghit Hit)
    (Rendering|Debug|DrawDebugPoint (.impactpoint Hit) 5.0 "(R=0.575000,G=0.000000,B=0.170499,A=1.000000)" 0.0)
    (CallFunction|ApplyFriction NormalImpulse (.impactpoint Hit) (.time Hit) (.impactnormal Hit) (Variables|Default|GetP2))))

(event OnComponentHit(P3)
  (params (OtherActor :type Actor%20Object%20Reference) (OtherComp :type Primitive%20Component%20Object%20Reference) (NormalImpulse :type Vector) (Hit :type Hit%20Result%20Structure%20%28by%20ref%29))
  (if (.bblockinghit Hit)
    (Rendering|Debug|DrawDebugPoint (.impactpoint Hit) 5.0 "(R=0.575000,G=0.000000,B=0.170499,A=1.000000)" 0.0)
    (CallFunction|ApplyFriction NormalImpulse (.impactpoint Hit) (.time Hit) (.impactnormal Hit) (Variables|Default|GetP3))))

(event OnComponentHit(P4)
  (params (OtherActor :type Actor%20Object%20Reference) (OtherComp :type Primitive%20Component%20Object%20Reference) (NormalImpulse :type Vector) (Hit :type Hit%20Result%20Structure%20%28by%20ref%29))
  (if (.bblockinghit Hit)
    (Rendering|Debug|DrawDebugPoint (.impactpoint Hit) 5.0 "(R=0.575000,G=0.000000,B=0.170499,A=1.000000)" 0.0)
    (CallFunction|ApplyFriction NormalImpulse (.impactpoint Hit) (.time Hit) (.impactnormal Hit) (Variables|Default|GetP4))))

(event OnComponentHit(Cube)
  (params (OtherActor :type Actor%20Object%20Reference) (OtherComp :type Primitive%20Component%20Object%20Reference) (NormalImpulse :type Vector) (Hit :type Hit%20Result%20Structure%20%28by%20ref%29))
  (if (.bblockinghit Hit)
    (Rendering|Debug|DrawDebugPoint (.impactpoint Hit) 5.0 "(R=0.575000,G=0.000000,B=0.170499,A=1.000000)" 0.0)))

(event OnComponentHit(P1)
  (params (OtherActor :type Actor%20Object%20Reference) (OtherComp :type Primitive%20Component%20Object%20Reference) (NormalImpulse :type Vector) (Hit :type Hit%20Result%20Structure%20%28by%20ref%29))
  (if (.bblockinghit Hit)
    (Rendering|Debug|DrawDebugPoint (.impactpoint Hit) 5.0 "(R=0.575000,G=0.000000,B=0.170499,A=1.000000)" 0.0)
    (CallFunction|ApplyFriction NormalImpulse (.impactpoint Hit) (.time Hit) (.impactnormal Hit) (Variables|Default|GetP1))))

(event EventBeginPlay)

(event Collision|EventActorBeginOverlap
  (params (OtherActor :type Actor%20Object%20Reference)))

(event EventTick
  (params (DeltaSeconds :type Float%20%28single-precision%29))
  (Utilities|FlowControl|Sequence
    (:then_0
      (bind _returnvalue (Physics|GetPhysicsLinearVelocity (Variables|Default|GetCube) "None"))
      (Rendering|Debug|DrawDebugString (Transformation|GetActorLocation) (Utilities|String|ToString(Vector) _returnvalue) 0 "(R=1.000000,G=1.000000,B=1.000000,A=1.000000)"))
    (:then_1
      (bind _returnvalue_2 (Class|PrimitiveComponent|GetPhysicsAngularVelocity (Variables|Default|GetCube) "None"))
      (Rendering|Debug|DrawDebugString (+ (Transformation|GetActorLocation) "0, 0,-20.000000") (Utilities|String|ToString(Vector) _returnvalue_2) 0 "(R=0.089102,G=0.070000,B=1.000000,A=1.000000)"))))

(event Input|ActionEvents|InputActionZoomIn
  (params (Key :type Key%20Structure :default "AnyKey"))
  (bind _springarm (Variables|Default|GetSpringArm))
  ;[1 1 1] Camera Control
  (:Pressed
    (Variables|/Script/Engine.SpringArmComponent|SetTargetArmLength _springarm (+ (Variables|/Script/Engine.SpringArmComponent|GetTargetArmLength _springarm) -25.0))))

(event Input|ActionEvents|InputActionZoomOut
  (params (Key :type Key%20Structure :default "AnyKey"))
  (bind _springarm (Variables|Default|GetSpringArm))
  ;[1 1 1] Camera Control
  (:Pressed
    (Variables|/Script/Engine.SpringArmComponent|SetTargetArmLength _springarm (+ (Variables|/Script/Engine.SpringArmComponent|GetTargetArmLength _springarm) 25.0))))

(event Input|KeyboardEvents|H
  (params (Key :type Key%20Structure :default "AnyKey"))
  (:Pressed
    (Class|PrimitiveComponent|AddForceatLocation (Variables|Default|GetCube) (Math|Transform|TransformDirection (Transformation|GetActorTransform) "200000.000000, 0, 0") (Transformation|GetWorldLocation (Variables|Default|GetF)) "None")))

(event Input|KeyboardEvents|B
  (params (Key :type Key%20Structure :default "AnyKey"))
  (bind _t1 (Variables|Default|GetT1))
  (bind _t2 (Variables|Default|GetT2))
  (bind _t3 (Variables|Default|GetT3))
  (bind _t4 (Variables|Default|GetT4))
  (bind _array (Utilities|Array|MakeArray _t1 _t2 _t3 _t4))
  (:Pressed
    (for _array_element _array
      (bind _returnvalue (Class|PrimitiveComponent|GetPhysicsLinearVelocityatPoint (Variables|Default|GetCube) (Transformation|GetWorldLocation _array_element) "None"))
      (Class|PrimitiveComponent|AddForceatLocation (Variables|Default|GetCube) (/ (* (* (* _returnvalue -1.0) (Physics|GetMass (Variables|Default|GetCube))) (/ 1.0 (Utilities|Time|GetWorldDeltaSeconds))) (Math|Conversions|ToFloat(Integer) (Utilities|Array|Length _array))) (Transformation|GetWorldLocation _array_element) "None"))))

(fn ConstructionScript)

(fn ApplyFriction
  (params (NormalImpulse :type Vector) (ContactPoint :type Vector) (HitTime :type Float%20%28single-precision%29) (SurfaceNormal :type Vector) (Component :type Static%20Mesh%20Component%20Object%20Reference))
  (Class|PrimitiveComponent|SetPhysMaterialOverride Component "/Game/Materials/NoFric_V2.NoFric_V2")
  (Class|PrimitiveComponent|SetPhysMaterialOverride (Variables|Default|GetCube) "/Game/Materials/FullFric.FullFric"))