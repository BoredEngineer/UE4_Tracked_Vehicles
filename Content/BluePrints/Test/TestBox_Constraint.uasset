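; Physics test box for experimenting with forces on a simulated Cube, with debug drawing and spring-arm camera zoom.
; H pushes the cube along local X; B applies velocity-cancelling forces split across four points.
; Blocking hits briefly lock the normally free PhysicsConstraint to sample its force, which also displays every tick.
; ApplyFriction computes surface-projected friction capped by normal impulse, but nothing here calls it; several other force experiments are disconnected.
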(event OnComponentHit(Cube)
  (params (OtherActor :type Actor%20Object%20Reference) (OtherComp :type Primitive%20Component%20Object%20Reference) (NormalImpulse :type Vector) (Hit :type Hit%20Result%20Structure%20%28by%20ref%29))
  (if (.bblockinghit Hit)
    (Rendering|Debug|DrawDebugPoint (.impactpoint Hit) 5.0 "(R=0.575000,G=0.000000,B=0.170499,A=1.000000)" 0.0)
    (CallFunction|SwitchConstraint true)
    (bind _outlinearforce (Class|PhysicsConstraintComponent|GetConstraintForce (Variables|Default|GetPhysicsConstraint)))
    (Rendering|Debug|DrawDebugString (+ (Transformation|GetActorLocation) "0, 0,100.000000") (Utilities|String|ToString(Vector) _outlinearforce) 0 "(R=0.984120,G=0.051053,B=1.000000,A=1.000000)")
    (CallFunction|SwitchConstraint false)))

(event EventBeginPlay
  (CallFunction|SwitchConstraint false))

(event Collision|EventActorBeginOverlap
  (params (OtherActor :type Actor%20Object%20Reference)))

(event EventTick
  (params (DeltaSeconds :type Float%20%28single-precision%29))
  (bind _outlinearforce (Class|PhysicsConstraintComponent|GetConstraintForce (Variables|Default|GetPhysicsConstraint)))
  (Rendering|Debug|DrawDebugString (+ (Transformation|GetActorLocation) "0, 0,100.000000") (Utilities|String|ToString(Vector) _outlinearforce) 0 "(R=0.984120,G=0.051053,B=1.000000,A=1.000000)"))

(event Input|ActionEvents|InputActionZoomIn
  (params (Key :type Key%20Structure :default "AnyKey"))
  (bind _springarm (Variables|Default|GetSpringArm))
  ;[1 1 1] Camera Control
  (:Pressed
    (Variables|/Script/Engine.SpringArmComponent|SetTargetArmLength _springarm (+ (Variables|/Script/Engine.SpringArmComponent|GetTargetArmLength _springarm) -25.0))))

(event Input|ActionEvents|InputActionZoomOut
  (params (Key :type Key%20Structure :default "AnyKey"))
  (bind _springarm (Variables|Default|GetSpringArm))
  ;[1 1 1] Camera Control
  (:Pressed
    (Variables|/Script/Engine.SpringArmComponent|SetTargetArmLength _springarm (+ (Variables|/Script/Engine.SpringArmComponent|GetTargetArmLength _springarm) 25.0))))

(event Input|KeyboardEvents|H
  (params (Key :type Key%20Structure :default "AnyKey"))
  (:Pressed
    (Class|PrimitiveComponent|AddForceatLocation (Variables|Default|GetCube) (Math|Transform|TransformDirection (Transformation|GetActorTransform) "200000.000000, 0, 0") (Transformation|GetWorldLocation (Variables|Default|GetF)) "None")))

(event Input|KeyboardEvents|B
  (params (Key :type Key%20Structure :default "AnyKey"))
  (bind _array (Utilities|Array|MakeArray 0 0 0 0))
  (:Pressed
    (for _array_element _array
      (bind _returnvalue (Class|PrimitiveComponent|GetPhysicsLinearVelocityatPoint (Variables|Default|GetCube) (Transformation|GetWorldLocation _array_element) "None"))
      (Class|PrimitiveComponent|AddForceatLocation (Variables|Default|GetCube) (/ (* (* (* _returnvalue -1.0) (Physics|GetMass (Variables|Default|GetCube))) (/ 1.0 (Utilities|Time|GetWorldDeltaSeconds))) (Math|Conversions|ToFloat(Integer) (Utilities|Array|Length _array))) (Transformation|GetWorldLocation _array_element) "None"))))

(fn ConstructionScript)

(fn ApplyFriction
  (params (NormalImpulse :type Vector) (ContactPoint :type Vector) (HitTime :type Float%20%28single-precision%29) (SurfaceNormal :type Vector))
  (bind _returnvalue (Class|PrimitiveComponent|GetPhysicsLinearVelocityatPoint (Variables|Default|GetCube) ContactPoint "None"))
  (if (> (Math|Vector|VectorLength _returnvalue) 5.0)
    (Class|PrimitiveComponent|AddForceatLocation (Variables|Default|GetCube) (Math|Vector|ClampVectorSize (Math|Vector|ProjectVectorontoPlane (/ (* (* (* _returnvalue -1.0) (Physics|GetMass (Variables|Default|GetCube))) (/ 1.0 (Utilities|Time|GetWorldDeltaSeconds))) 4.0) SurfaceNormal) 0.0 (* (* (Math|Vector|VectorLength NormalImpulse) (/ 1.0 (Utilities|Time|GetWorldDeltaSeconds))) 0.6)) ContactPoint "None")
    (Rendering|Debug|DrawDebugLine ContactPoint (+ ContactPoint NormalImpulse) "(R=0.182015,G=0.110873,B=0.935000,A=1.000000)" 0.0 5.0)
    (Rendering|Debug|DrawDebugLine :LineStart ContactPoint :LineEnd (+ ContactPoint (Math|Vector|ClampVectorSize (Math|Vector|ProjectVectorontoPlane (/ (* (* (* _returnvalue -1.0) (Physics|GetMass (Variables|Default|GetCube))) (/ 1.0 (Utilities|Time|GetWorldDeltaSeconds))) 4.0) SurfaceNormal) 0.0 (* (* (Math|Vector|VectorLength NormalImpulse) (/ 1.0 (Utilities|Time|GetWorldDeltaSeconds))) 0.6))) :Thickness 5.0)))

(fn SwitchConstraint
  (params (SwitchedOn :type Boolean))
  (bind _physicsconstraint (Variables|Default|GetPhysicsConstraint))
  (if SwitchedOn
    (Class|PhysicsConstraintComponent|SetLinearXLimit _physicsconstraint "LCM_Locked" 0.0)
    (Class|PhysicsConstraintComponent|SetLinearYLimit _physicsconstraint "LCM_Locked" 0.0)
    (Class|PhysicsConstraintComponent|SetLinearZLimit _physicsconstraint "LCM_Locked" 0.0)
    (else
      (Class|PhysicsConstraintComponent|SetLinearXLimit _physicsconstraint "LCM_Free" 0.0)
      (Class|PhysicsConstraintComponent|SetLinearYLimit _physicsconstraint "LCM_Free" 0.0)
      (Class|PhysicsConstraintComponent|SetLinearZLimit _physicsconstraint "LCM_Free" 0.0))))